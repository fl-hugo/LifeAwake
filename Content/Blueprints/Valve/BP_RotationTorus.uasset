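; BP_RotationTorus is a rotating object that spins in yaw when the BP_Valve that owns it signals a valve rotation.
; On BeginPlay it casts its owner to BP_Valve and binds Rotate to that event.
; Rotate plays a timeline that sets absolute world yaw to the curve value times RotationValue, preserving roll and pitch.
; An IsRotating flag ignores new triggers until the timeline finishes, with debug prints at start and end.
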(event Custom|Rotate
  (bind _defaultsceneroot (Variables|Default|GetDefaultSceneRoot))
  (bind _returnvalue (Transformation|GetWorldRotation _defaultsceneroot))
  (if (not (Variables|Default|GetisRotating))
    (Variables|Default|SetisRotating true)
    (Development|PrintString "StartRotating")
    (bind _rotationvalue (Timeline|RotationTimeline PlayFromStart)
      (:Update
        (Transformation|SetWorldRotation (Variables|Default|GetDefaultSceneRoot) (Math|Rotator|MakeRotator (.roll _returnvalue) (.pitch _returnvalue) (* _rotationvalue (Variables|Default|GetRotationValue))) false false))
      (:Finished
        (Variables|Default|SetisRotating false)
        (Development|PrintString "End rotating")))))

(event EventBeginPlay
  (bind _asbp_valve (Utilities|Casting|CastToBP_Valve (Components|GetOwner)))
  (EventDispatchers|BindEventtoValveRotation _asbp_valve (delegate Custom|Rotate)))

(fn ConstructionScript)