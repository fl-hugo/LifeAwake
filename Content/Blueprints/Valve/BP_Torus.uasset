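; BP_Torus is the torus piece of a valve, turning about its yaw axis when its parent BP_Valve signals a rotation.
; On BeginPlay it casts its parent actor to BP_Valve, binds to the rotation event and copies the valve's RotationValue.
; A timeline scales that value and adds it to the starting world yaw, while a flag ignores new triggers until the turn finishes.
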(event Custom|Rotate
  (bind _defaultsceneroot (Variables|Default|GetDefaultSceneRoot))
  (bind _returnvalue (Transformation|GetWorldRotation _defaultsceneroot))
  ;[1 1 1] Rotation
  (if (not (Variables|Default|GetisRotating))
    (Variables|Default|SetYaw%20rotation (.yaw (Transformation|GetWorldRotation (Variables|Default|GetDefaultSceneRoot))))
    (Variables|Default|SetisRotating true)
    (bind _rotationvalue (Timeline|RotationTimeline PlayFromStart)
      (:Update
        (Transformation|SetWorldRotation (Variables|Default|GetDefaultSceneRoot) (Math|Rotator|MakeRotator (.roll _returnvalue) (.pitch _returnvalue) (+ (* _rotationvalue (Variables|Default|GetRotationValue)) (Variables|Default|GetYaw%20rotation))) false false))
      (:Finished
        (Variables|Default|SetisRotating false)))))

(event EventBeginPlay
  ;[1 1 1] Biding
  (bind _asbp_valve (Utilities|Casting|CastToBP_Valve (Actor|GetParentActor)))
  (EventDispatchers|BindEventtoValveRotation _asbp_valve (delegate Custom|Rotate))
  (Variables|Default|SetRotationValue (Variables|/Game/Blueprints/Valve/BP_Valve.BP_Valve_C|GetRotationValue _asbp_valve)))

(fn ConstructionScript)