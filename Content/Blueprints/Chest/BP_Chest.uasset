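; BP_Chest is an interactable chest that checks the game instance's inventory for BP_Key when used.
; With the key, it prints a placeholder animation message, forwards the interaction to its BPClue child actor, removes the key and toggles State.
; Without the key, a true State still runs that same clue, removal and toggle path, while a false State prints a no-key message.
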(event EventObjectInteraction
  (if (== (Utilities|Array|FindItem (Variables|/Game/Blueprints/BP_BasicGameInstance.BP_BasicGameInstance_C|GetInventory (CallFunction|GetGameInstance)) "/Game/Blueprints/Chest/BP_Key.BP_Key_C") -1)
    (if (Variables|Default|GetState)
      (Class|IInteraction|ObjectInteraction(Message) (Variables|/Script/Engine.ChildActorComponent|GetChildActor (Variables|Default|GetBP_Clue)) :!label _label)
      (Utilities|Array|RemoveItem (Variables|/Game/Blueprints/BP_BasicGameInstance.BP_BasicGameInstance_C|GetInventory (CallFunction|GetGameInstance)) "/Game/Blueprints/Chest/BP_Key.BP_Key_C")
      (CallFunction|Toggle)
      (else
        (Development|PrintString "no key")))
    (else
      (Development|PrintString "Play chest animation")
      (goto _label))))

(fn ConstructionScript)

(fn Toggle
  (Variables|Default|SetState (not (Variables|Default|GetState))))