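; AC_Music is an actor component that sets the background music for the current level when play begins.
; It picks one track for the Hub level and another for all other levels.
; The audio component is kept on the GameInstance: if valid, its sound is swapped only when different.
; Otherwise it spawns a 2D sound at the GameInstance's music volume and stores that reference.
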(event EventBeginPlay
  (bind _gameinstanceref (CallFunction|GetGameInstance))
  (bind _returnvalue (Game|GetCurrentLevelName true))
  (Utilities|IsValid (Variables|/Game/Blueprints/BP_BasicGameInstance.BP_BasicGameInstance_C|GetAudio (CallFunction|GetGameInstance))
    (:Is%20Valid
      (if (!= (Variables|/Script/Engine.AudioComponent|GetSound (Variables|/Game/Blueprints/BP_BasicGameInstance.BP_BasicGameInstance_C|GetAudio (CallFunction|GetGameInstance))) (select (Utilities|Enum|Equal(Enum) _returnvalue "Hub") "/Game/Audio/Life_Awake_-_Level_Glace.Life_Awake_-_Level_Glace" "/Game/Audio/raf_desert.raf_desert"))
        (Audio|Components|Audio|SetSound (Variables|/Game/Blueprints/BP_BasicGameInstance.BP_BasicGameInstance_C|GetAudio (CallFunction|GetGameInstance)) (select (Utilities|Enum|Equal(Enum) _returnvalue "Hub") "/Game/Audio/Life_Awake_-_Level_Glace.Life_Awake_-_Level_Glace" "/Game/Audio/raf_desert.raf_desert")) ; set new sound if sound not already playing
      ))
    (:Is%20Not%20Valid
      ;[0.15 0.15 0.15 0.5] Create Sound 2D for first time
      (bind _returnvalue_2 (Audio|SpawnSound2D (select (Utilities|Enum|Equal(Enum) _returnvalue "Hub") "/Game/Audio/Life_Awake_-_Level_Glace.Life_Awake_-_Level_Glace" "/Game/Audio/raf_desert.raf_desert") (Variables|/Game/Blueprints/BP_BasicGameInstance.BP_BasicGameInstance_C|GetMusicVolume _gameinstanceref) 1.0 0.0 0 true))
      (Variables|/Game/Blueprints/BP_BasicGameInstance.BP_BasicGameInstance_C|SetAudio _gameinstanceref _returnvalue_2))))