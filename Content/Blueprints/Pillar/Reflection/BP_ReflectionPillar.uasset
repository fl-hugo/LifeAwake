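; BP_ReflectionPillar is a pillar that rotates in yaw by a set step when interacted with, if rotation is allowed and none is in progress.
; A timeline drives the turn from the current yaw, and dispatchers signal its start and stop.
; BeginPlay can offset the starting yaw by a random number of steps.
; A helper returns the first BP_LightCreator in the level, and the construction script's mesh and material setup is disconnected.
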(event EventBeginPlay
  (bind _returnvalue (Transformation|GetActorRotation))
  (if (Variables|Default|GetDoesRandomRotate)
    (Transformation|SetActorRotation (Math|Rotator|MakeRotator (.roll _returnvalue) (.pitch _returnvalue) (+ (.yaw _returnvalue) (* (Class|KismetMathLibrary|RandomInteger64inRange 0 5) (Variables|Default|GetRotationValue)))))))

(event EventObjectInteraction
  (bind _defaultsceneroot (Variables|Default|GetDefaultSceneRoot))
  (bind _returnvalue (Transformation|GetWorldRotation _defaultsceneroot))
  (if (Variables|Default|GetCanBeRotate)
    (if (not (Variables|Default|GetisRotating))
      (Variables|Default|SetYawRotation (.yaw (Transformation|GetWorldRotation (Variables|Default|GetDefaultSceneRoot))))
      (Variables|Default|SetisRotating true)
      (Default|CallOnStartRotating)
      (bind _rotation (Timeline|Timeline PlayFromStart)
        (:Update
          (Transformation|SetWorldRotation (Variables|Default|GetDefaultSceneRoot) (Math|Rotator|MakeRotator (.roll _returnvalue) (.pitch _returnvalue) (+ (* _rotation (Variables|Default|GetRotationValue)) (Variables|Default|GetYawRotation))) false false))
        (:Finished
          (Variables|Default|SetisRotating false)
          (Default|CallOnStopRotating))))))

(fn ConstructionScript)

(fn GetLightCreator
  (bind _outactors (Actor|GetAllActorsOfClass "/Game/Blueprints/Pillar/Reflection/BP_LightCreator.BP_LightCreator_C"))
  (return (Utilities|Array|Get(acopy) _outactors)))