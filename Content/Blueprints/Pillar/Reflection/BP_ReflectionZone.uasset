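; BP_ReflectionZone is a reflective surface in a light-beam mechanic that bounces incoming light toward other zones.
; ReflectLight computes the mirror vector from the incident direction and normal, then traces on Visibility at impact height with debug drawing.
; The trace end uses the scaled reflection's X and Y directly, without adding the impact point.
; Hits on another reflection zone recursively call ReflectLight, while hits on a BP_LightTargetZone call LightHit.
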(event Custom|ReflectLight
  (params (ImpactPoint :type Vector) (Normal :type Vector) (TraceStart :type Vector))
  (Variables|Default|SetIncident (Math|Vector|Normalize (- ImpactPoint TraceStart)))
  (Variables|Default|SetNormal (Math|Vector|Normalize Normal))
  (bind _output_get (Variables|Default|SetReflection (- (Variables|Default|GetIncident) (* (* (Math|Vector|DotProduct (Variables|Default|GetNormal) (Variables|Default|GetIncident)) 2.0) (Variables|Default|GetNormal)))))
  (bind _outhit (Collision|LineTraceByChannel ImpactPoint (Math|Vector|MakeVector (.x (* _output_get 1e+04)) (.y (* _output_get 1e+04)) (.Z (Math|Vector|BreakVector ImpactPoint))) "TraceTypeQuery1" false 0 "ForOneFrame" true "(R=0.200449,G=0.733953,B=1.000000,A=1.000000)" "(R=0.000000,G=1.000000,B=0.000000,A=0.000000)"))
  (bind _asbp_reflection_zone (Utilities|Casting|CastToBP_ReflectionZone (.HitActor (Collision|BreakHitResult _outhit)))
    (:then
      (CallFunction|ReflectLight _asbp_reflection_zone (.ImpactPoint (Collision|BreakHitResult _outhit)) (.Normal (Collision|BreakHitResult _outhit)) (.TraceStart (Collision|BreakHitResult _outhit))))
    (:CastFailed
      (bind _asbp_light_target_zone (Utilities|Casting|CastToBP_LightTargetZone (.HitActor (Collision|BreakHitResult _outhit))))
      (Default|LightHit _asbp_light_target_zone))))

(fn ConstructionScript)