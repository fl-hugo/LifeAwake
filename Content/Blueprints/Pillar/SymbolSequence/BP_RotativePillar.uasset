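; Rotating four-symbol pillar, apparently for a symbol-sequence puzzle, that turns by a set yaw step when interacted with.
; A timeline animates each turn and blocks further interaction until it finishes.
; An optional random start rotation is saved at BeginPlay for the reset event to restore.
; GetCurrentSymbol maps the actor's yaw quadrant to a BP_PillarSymbol child actor and returns its symbol name.
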(event Custom|ResetPillarPosition
  ;[1 1 1] Reset pillar position
  (Transformation|SetActorRotation (Math|Rotator|MakeRotator 0.0 0.0 (Variables|Default|GetZRotation))))

(event EventBeginPlay
  (bind _returnvalue (Transformation|GetActorRotation))
  ;[1 1 1] Random rotation at start
  (if (Variables|Default|GetDoesRandomRotate)
    (Transformation|SetActorRotation (Math|Rotator|MakeRotator (.roll _returnvalue) (.pitch _returnvalue) (+ (.yaw _returnvalue) (* (Class|KismetMathLibrary|RandomInteger64inRange 0 5) (Variables|Default|GetRotationValue)))))
    (Variables|Default|SetZRotation (.yaw (Transformation|GetActorRotation)))))

(event EventObjectInteraction
  (bind _defaultsceneroot (Variables|Default|GetDefaultSceneRoot))
  (bind _returnvalue (Transformation|GetWorldRotation _defaultsceneroot))
  ;[1 1 1] Rotation management
  (if (not (Variables|Default|GetisRotating))
    (Variables|Default|SetYawRotation (.yaw (Transformation|GetWorldRotation (Variables|Default|GetDefaultSceneRoot))))
    (Variables|Default|SetisRotating true)
    (bind _rotation (Timeline|Timeline PlayFromStart)
      (:Update
        (Transformation|SetWorldRotation (Variables|Default|GetDefaultSceneRoot) (Math|Rotator|MakeRotator (.roll _returnvalue) (.pitch _returnvalue) (+ (* _rotation (Variables|Default|GetRotationValue)) (Variables|Default|GetYawRotation))) false false))
      (:Finished
        (Variables|Default|SetisRotating false)))))

(fn ConstructionScript)

(fn GetCurrentSymbol
  (switch int (/ (Math|Float|Truncate (.yaw (Transformation|GetActorRotation self))) 90)
    (:-1
      (bind _symbolname (CallFunction|GetSymbolName (Variables|Default|GetSymbol3)))
      (LocalVariables|SetCurrentSymbol _symbolname))
    (:0
      (bind _symbolname_2 (CallFunction|GetSymbolName (Variables|Default|GetSymbol4)))
      (LocalVariables|SetCurrentSymbol _symbolname_2))
    (:1
      (bind _symbolname_3 (CallFunction|GetSymbolName (Variables|Default|GetSymbol1)))
      (LocalVariables|SetCurrentSymbol _symbolname_3))
    (:2
      (bind _symbolname_4 (CallFunction|GetSymbolName (Variables|Default|GetSymbol2)))
      (LocalVariables|SetCurrentSymbol _symbolname_4)))
  (return (LocalVariables|GetCurrentSymbol)))

(fn GetSymbolName
  (params (Child%20Actor :type Child%20Actor%20Component%20Object%20Reference))
  (bind _asbp_pillar_symbol (Utilities|Casting|CastToBP_PillarSymbol (Variables|/Script/Engine.ChildActorComponent|GetChildActor Child%20Actor)))
  (return (Variables|/Game/Blueprints/Pillar/SymbolSequence/BP_PillarSymbol.BP_PillarSymbol_C|GetSymbolName _asbp_pillar_symbol)))