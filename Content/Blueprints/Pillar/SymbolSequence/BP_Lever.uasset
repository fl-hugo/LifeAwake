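; BP_Lever is an interactable lever for the pillar symbol-sequence puzzle that triggers pillar verification when used.
; ObjectInteraction checks and clears a CanBeUsed flag, starts the lever animation and immediately calls CallVerifyPillars.
; A timeline drives the lever's world pitch, then reverses on finish to return it, re-enabling interaction as the return begins.
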(event Custom|LeverAnimation
  ;[1 1 1] Lever Animations
  (bind _leverrotation (Timeline|T_Activate PlayFromStart)
    (:Update
      (Transformation|SetWorldRotation (Variables|Default|GetLever) (Math|Rotator|MakeRotator 0.0 (* _leverrotation 35.0) 0.0) false false))
    (:Finished
      (CallFunction|LeverReverseAnimation)
      (Variables|Default|SetCanBeUsed true))))

(event Custom|LeverReverseAnimation
  ;[1 1 1] Lever Animations
  (bind _leverrotation (Timeline|T_Activate Reverse)
    (:Update
      (Transformation|SetWorldRotation (Variables|Default|GetLever) (Math|Rotator|MakeRotator 0.0 (* _leverrotation 35.0) 0.0) false false))
    (:Finished
      (CallFunction|LeverReverseAnimation)
      (Variables|Default|SetCanBeUsed true))))

(event EventObjectInteraction
  ;[1 1 1] Interaction
  (if (Variables|Default|GetCanBeUsed)
    (Variables|Default|SetCanBeUsed false)
    (CallFunction|LeverAnimation)
    (Default|CallVerifyPillars)))

(fn ConstructionScript)