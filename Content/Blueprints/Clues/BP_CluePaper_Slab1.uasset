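; BP_CluePaper_Slab1 is an interactable clue paper that shows its text and image to the player.
; On interaction it creates a WB_CluePaper widget from its clue text and texture and passes it to the pause component with the cursor hidden.
; It then toggles its State flag, and when that flag becomes false it adds its class to the inventory component and destroys itself.
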(event EventObjectInteraction
  (bind _returnvalue (UserInterface|CreateWidget "/Game/Widgets/WB_CluePaper.WB_CluePaper_C" 0 (Variables|Default|GetClueText) (Variables|Default|GetClue%20Texture) "" 0))
  (Default|Pause (Variables|Default|GetAC_Pause) 0 _returnvalue false)
  (CallFunction|Toggle)
  (if (not (Variables|Default|GetState))
    (Default|AddtoInventory (Variables|Default|GetAC_Inventory) (Utilities|GetClass self))
    (Actor|DestroyActor)))

(fn ConstructionScript)

(fn Toggle
  (Variables|Default|SetState (not (Variables|Default|GetState))))