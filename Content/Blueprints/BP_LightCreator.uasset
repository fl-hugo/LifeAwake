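; BP_LightCreator is a light beam emitter that casts a line trace along its forward vector every tick.
; SpawnLight runs a Visibility trace with persistent debug drawing between the given start and end points.
; When the trace hits a BP_ReflectionZone, it passes the impact point, surface normal and trace start to that zone's ReflectLight.
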(event Custom|SpawnLight
  (params (Start :type Vector) (End :type Vector))
  (bind _outhit (Collision|LineTraceByChannel Start End "TraceTypeQuery1" false 0 "Persistent" true "(R=0.200449,G=0.733953,B=1.000000,A=1.000000)" "(R=0.000000,G=1.000000,B=0.000000,A=0.000000)"))
  (bind _asbp_reflection_zone (Utilities|Casting|CastToBP_ReflectionZone (.HitActor (Collision|BreakHitResult _outhit))))
  (Default|ReflectLight _asbp_reflection_zone (.ImpactPoint (Collision|BreakHitResult _outhit)) (.Normal (Collision|BreakHitResult _outhit)) (.TraceStart (Collision|BreakHitResult _outhit))))

(event EventTick
  (params (DeltaSeconds :type Float%20%28single-precision%29))
  (bind _returnvalue (Transformation|GetActorLocation))
  (CallFunction|SpawnLight _returnvalue (+ (* (Math|Vector|GetForwardVector (Transformation|GetActorRotation)) 1e+03) _returnvalue)))

(fn ConstructionScript)