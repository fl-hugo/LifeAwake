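; BP_Tree is a tree actor whose trunk mesh can be swapped at runtime, with foliage and materials updated to match.
; SetMesh assigns the trunk mesh, then uses lookup maps keyed by mesh to pick the leaves mesh and both materials.
; A transform map moves the root in world space, and one hard-coded case offsets the foliage for the Second_tree_low mesh.
; Missing leaf or material entries print a debug string.
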(event Custom|SetMesh
  (params (NewMesh :type Static%20Mesh%20Object%20Reference))
  (bind _sm_tree (Variables|Default|GetSM_Tree))
  (Components|StaticMesh|SetStaticMesh _sm_tree NewMesh)
  (CallFunction|SetMaterial (Variables|/Script/Engine.StaticMeshComponent|GetStaticMesh _sm_tree) (Variables|Default|GetSM_Tree))
  (CallFunction|SetFoliageMesh)
  (CallFunction|SetTransform)
  (CallFunction|SetFoliageTransform))

(fn ConstructionScript)

(fn SetFoliageMesh
  (bind _leavesmapping (LocalVariables|GetLeavesMapping))
  (bind _sm_tree (Variables|Default|GetSM_Tree))
  (bind _staticmesh (Variables|/Script/Engine.StaticMeshComponent|GetStaticMesh _sm_tree))
  (bind (_value _returnvalue) (Utilities|Map|Find _leavesmapping _staticmesh))
  (if _returnvalue
    (Components|StaticMesh|SetStaticMesh (Variables|Default|GetSM_Foliage) _value)
    (CallFunction|SetMaterial _value (Variables|Default|GetSM_Foliage))
    (else
      (Development|PrintString "Leave doesn't found"))))

(fn SetMaterial
  (params (StaticMesh :type Static%20Mesh%20Object%20Reference) (MeshTarget :type Primitive%20Component%20Object%20Reference))
  (bind _materialmapping (LocalVariables|GetMaterialMapping))
  (bind (_value _returnvalue) (Utilities|Map|Find _materialmapping StaticMesh))
  (if _returnvalue
    (Rendering|Material|SetMaterial MeshTarget 0 _value)
    (else
      (Development|PrintString "Material doesn't found"))))

(fn SetTransform
  (bind _sm_tree (Variables|Default|GetSM_Tree))
  (bind _transformmapping (LocalVariables|GetTransformMapping))
  (bind _staticmesh (Variables|/Script/Engine.StaticMeshComponent|GetStaticMesh _sm_tree))
  (bind (_value _returnvalue) (Utilities|Map|Find _transformmapping _staticmesh))
  (if _returnvalue
    (Transformation|SetWorldTransform (Variables|Default|GetDefaultSceneRoot) _value false false)))

(fn SetFoliageTransform
  (if (== (Variables|/Script/Engine.StaticMeshComponent|GetStaticMesh (Variables|Default|GetSM_Tree)) "/Game/3D_Part/LIFE_AWAKE/props/second_tree_low.second_tree_low")
    (Transformation|SetRelativeLocation (Variables|Default|GetSM_Foliage) "5.300000,0.000000,53.000000" false false)))