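; FL_Game is a function library of game-wide lookup helpers for the game instance and item data.
; GetGameInstance returns the game instance cast to BP_BasicGameInstance.
; GetItemClass and GetItemTexture look up a named row in a supplied DataTable and return its Actor or Texture field, respectively.
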(fn GetGameInstance
  (bind _asbp_basic_game_instance (Utilities|Casting|CastToBP_BasicGameInstance (Game|GetGameInstance)))
  (return _asbp_basic_game_instance))

(fn GetItemClass
  (params (DataTable :type Data%20Table%20Object%20Reference) (Name :type Name))
  (bind _returnvalue (Utilities|GetDataTableRow DataTable Name)
    (:then
      (return (.Actor (Utilities|Struct|BreakS_Item _returnvalue))))))

(fn GetItemTexture
  (params (DataTable :type Data%20Table%20Object%20Reference) (Name :type Name))
  (bind _returnvalue (Utilities|GetDataTableRow DataTable Name)
    (:then
      (return (.Texture (Utilities|Struct|BreakS_Item _returnvalue))))))