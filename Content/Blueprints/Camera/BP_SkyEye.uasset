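; BP_SkyEye is an alternate camera view that the IA_SkyEye input toggles against the player character's view.
; A Player/SkyEye/Switching state machine, with empty enter and exit hooks, blocks new switches during the eased view-target blend.
; A timer matching the blend time sets the destination state and subscribes to character movement updates.
; The first detected movement unsubscribes and, in SkyEye, blends back to the player.
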(event Custom|EndSwitch
  (CallFunction|ChangeState (CallFunction|TargetState))
  (OneTimeCheck|ToggleMovementCheck true))

(event Input|EnhancedActionEvents|EnhancedInputActionIA_SkyEye
  (params (ActionValue :type Boolean) (ElapsedSeconds :type Float%20%28double-precision%29) (TriggeredSeconds :type Float%20%28double-precision%29) (InputAction :type Input%20Action%20Object%20Reference :default "/Game/Input/Actions/IA_SkyEye.IA_SkyEye"))
  (CallFunction|Switch (Utilities|Enum|Equal(Enum) (Variables|Default|GetState) "NewEnumerator2")))

(event EventBeginPlay
  (CallFunction|ChangeState "NewEnumerator0"))

(fn ConstructionScript)

(fn NotNearlyZero
  (params (A :type Vector%20%28by%20ref%29))
  (return (not (Math|Vector|VectorIsNearlyZero A))))

(fn ToggleMovementCheck
  (params (Subscribe :type Boolean))
  (bind _returnvalue (Game|GetPlayerCharacter 0))
  (bind _output_get (Variables|Default|SetisSubscribed Subscribe))
  (if _output_get
    (Character|BindEventtoOnCharacterMovementUpdated _returnvalue (EventDispatchers|CreateEvent :!event OnMove))
    (return)
    (else
      (Character|UnbindEventfromOnCharacterMovementUpdated _returnvalue (EventDispatchers|CreateEvent :!event OnMove))
      (return))))

(fn OnMove
  (params (DeltaSeconds :type Float%20%28single-precision%29) (OldLocation :type Vector) (OldVelocity :type Vector))
  (if (Vector|NotNearlyZero OldVelocity)
    (OneTimeCheck|ToggleMovementCheck false)
    (if (Utilities|Enum|Equal(Enum) (Variables|Default|GetState) "NewEnumerator2")
      (CallFunction|Switch true))))

(fn ChangeState
  (params (State :type E_CameraState%20Enum :default "NewEnumerator0"))
  (if (Utilities|Enum|NotEqual(Enum) State (Variables|Default|GetState))
    (Utilities|FlowControl|Sequence
      (:then_0
        ;[0.15 0.15 0.15 0.5] Exit State
        (switch Utilities|FlowControl|Switch|SwitchonE_CameraState (Variables|Default|GetState)))
      (:then_1
        (bind _output_get (Variables|Default|SetState State :!label _label))
        ;[0.15 0.15 0.15 0.5] Enter State
        (switch Utilities|FlowControl|Switch|SwitchonE_CameraState _output_get)))
    (else
      (goto _label))))

(fn Switch
  (params (PlayerCamera :type Boolean))
  (if (not (CallFunction|IsSwitching))
    (bind _output_get (Variables|Default|SettoPlayerCamera PlayerCamera))
    (Game|Player|SetViewTargetwithBlend (Game|GetPlayerController 0) (CallFunction|TargetActor _output_get) (Variables|Default|GetBlendTime) "VTBlend_EaseInOut" 2.0 true)
    (CallFunction|ChangeState "NewEnumerator1")
    (Utilities|Time|SetTimerbyEvent (EventDispatchers|CreateEvent :!event Custom|EndSwitch) (Variables|Default|GetBlendTime))))

(fn IsSwitching
  (return (Utilities|Enum|Equal(Enum) (Variables|Default|GetState) "NewEnumerator1")))

(fn TargetState
  (return (select (Variables|Default|GettoPlayerCamera) "NewEnumerator0" "NewEnumerator2")))

(fn TargetActor
  (params (Index :type Boolean))
  (return (select Index (Game|GetPlayerCharacter 0) self)))