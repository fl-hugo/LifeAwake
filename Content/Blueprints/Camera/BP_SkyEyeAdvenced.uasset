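; Sky-eye camera actor that toggles the view between the player character and its own overhead camera on the IA_SkyEye input.
; A Player/Switching/SkyEye state ignores requests mid-blend, while a timer ends each SetViewTargetWithBlend transition.
; After each switch it watches character movement, and the first movement blends back to the player, with blend time capped by Maptime.
; Tick prints the current state for debugging.
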(event Custom|OnMoved
  (if (Utilities|Enum|NotEqual(Enum) (Variables|Default|GetState) "NewEnumerator1")
    (CallFunction|Switch true)))

(event Custom|EndSwitch
  (CallFunction|ChangeState (CallFunction|TargetState))
  (OneTimeCheck|ToggleMovementCheck true))

(event Input|EnhancedActionEvents|EnhancedInputActionIA_SkyEye
  (params (ActionValue :type Boolean) (ElapsedSeconds :type Float%20%28double-precision%29) (TriggeredSeconds :type Float%20%28double-precision%29) (InputAction :type Input%20Action%20Object%20Reference :default "/Game/Input/Actions/IA_SkyEye.IA_SkyEye"))
  (if (Utilities|Enum|NotEqual(Enum) (Variables|Default|GetState) "NewEnumerator1")
    (CallFunction|Switch (Utilities|Enum|Equal(Enum) (Variables|Default|GetState) "NewEnumerator2"))))

(event EventBeginPlay
  (CallFunction|ChangeState "NewEnumerator0")
  (EventDispatchers|BindEventtoOnPlayerStartMoving (EventDispatchers|CreateEvent :!event Custom|OnMoved)))

(event EventTick
  (params (DeltaSeconds :type Float%20%28single-precision%29))
  (Development|PrintString (Utilities|String|Append "STATE: " (Utilities|String|EnumtoString (Variables|Default|GetState))) true false "(R=0.000000,G=0.660000,B=1.000000,A=1.000000)" DeltaSeconds "STATE"))

(fn ConstructionScript)

(fn CalcBlendTime
  (params (toPlayer :type Boolean))
  (bind _blendtime (Variables|Default|GetBlendTime))
  (return (select toPlayer (Class|KismetMathLibrary|GetMin2D (Math|Vector2D|MakeVector2D _blendtime (|maptime))) _blendtime)))

(fn NotNearlyZero
  (params (A :type Vector%20%28by%20ref%29))
  (return (not (Math|Vector|VectorIsNearlyZero A))))

(fn ToggleMovementCheck
  (params (Subscribe :type Boolean))
  (bind _returnvalue (Game|GetPlayerCharacter 0))
  (bind _output_get (Variables|Default|SetisSubscribed Subscribe))
  (if _output_get
    (Character|BindEventtoOnCharacterMovementUpdated _returnvalue (EventDispatchers|CreateEvent :!event OnMove))
    (return)
    (else
      (Character|UnbindEventfromOnCharacterMovementUpdated _returnvalue (EventDispatchers|CreateEvent :!event OnMove))
      (return))))

(fn OnMove
  (params (DeltaSeconds :type Float%20%28single-precision%29) (OldLocation :type Vector) (OldVelocity :type Vector))
  (if (Vector|NotNearlyZero OldVelocity)
    (OneTimeCheck|ToggleMovementCheck false)
    (Default|CallOnPlayerStartMoving)))

(fn ChangeState
  (params (State :type E_CameraState%20Enum :default "NewEnumerator0"))
  (if (Utilities|Enum|NotEqual(Enum) State (Variables|Default|GetState))
    (Utilities|FlowControl|Sequence
      (:then_0
        ;[0.15 0.15 0.15 0.5] Exit State
        (switch Utilities|FlowControl|Switch|SwitchonE_CameraState (Variables|Default|GetState)))
      (:then_1
        (bind _output_get (Variables|Default|SetState State :!label _label))
        ;[0.15 0.15 0.15 0.5] Enter State
        (switch Utilities|FlowControl|Switch|SwitchonE_CameraState _output_get
          (:NewEnumerator1
            (Variables|Default|SetStartTime (Utilities|Time|GetGameTimeinSeconds))))))
    (else
      (goto _label))))

(fn Switch
  (params (PlayerCamera :type Boolean))
  (bind _output_get (Variables|Default|SettoPlayerCamera PlayerCamera))
  (bind _output_get_2 (Variables|Default|SetCalculatedBlendTime (Camera|CalcBlendTime _output_get)))
  (Game|Player|SetViewTargetwithBlend (Game|GetPlayerController 0) (CallFunction|TargetActor _output_get) _output_get_2 (select _output_get "VTBlend_Cubic" "VTBlend_EaseInOut") 2.0 true)
  (CallFunction|ChangeState "NewEnumerator1")
  (if (> (Variables|Default|GetCalculatedBlendTime) 0.0)
    _
    (else
      (CallFunction|EndSwitch)))
  (Utilities|Time|SetTimerbyEvent (EventDispatchers|CreateEvent :!event Custom|EndSwitch) (Variables|Default|GetCalculatedBlendTime)))

(fn IsSwitching
  (return (Utilities|Enum|Equal(Enum) (Variables|Default|GetState) "NewEnumerator1")))

(fn TargetState
  (return (select (Variables|Default|GettoPlayerCamera) "NewEnumerator0" "NewEnumerator2")))

(fn TargetActor
  (params (Index :type Boolean))
  (return (select Index (Game|GetPlayerCharacter 0) self)))

(fn IsBlended
  (bind _returnvalue (Game|GetPlayerController 0))
  (bind (_location _rotation) (Pawn|GetPlayerViewPoint _returnvalue))
  (bind _returnvalue_2 (Pawn|GetViewTarget _returnvalue))
  (bind _returnvalue_3 (Actor|GetComponentbyClass _returnvalue_2 "/Script/Engine.CameraComponent"))
  (return (and (Utilities|Operators|EqualEqual (Transformation|GetWorldLocation _returnvalue_3) _location 5e+01) (Utilities|Operators|EqualEqual (Transformation|GetWorldRotation _returnvalue_3) _rotation 5e+01))))

(fn MapDuration
  (params (Starting :type Vector) (Ending :type Vector) (Current :type Vector) (MaxDuration :type Float%20%28double-precision%29))
  ;[0.15 0.15 0.15 0.5] low2 + (high2 - low2) * (value - low1) / (high1 - low1)
  (return (/ (* MaxDuration (Math|Vector|VectorLength (- Current Starting))) (Math|Vector|VectorLength (- Ending Starting)))))

(fn BlendDuration
  (bind _duration (CallFunction|MapDuration (Transformation|GetWorldLocation (Actor|GetComponentbyClass (Game|GetPlayerCharacter 0) "/Script/Engine.CameraComponent")) (Transformation|GetWorldLocation (Variables|Default|GetCamera)) (.Location (Pawn|GetPlayerViewPoint (Game|GetPlayerController 0))) 1e+01))
  (return _duration))