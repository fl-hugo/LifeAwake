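; BP_CluePaper is an interactable clue paper that shows its clue text in a UI widget.
; On Interact, it creates a WB_CluePaper widget with its ClueText and hands it to ACPause's Pause with the cursor hidden.
; An older viewport show/hide path using the IsWidgetInViewport flag and Toggle function remains in the graph but never runs.
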(event EventInteract
  (bind _returnvalue (UserInterface|CreateWidget "/Game/Widgets/WB_CluePaper.WB_CluePaper_C" 0 (Variables|Default|GetClueText)))
  (Default|Pause (Variables|Default|GetAC_Pause) 0 _returnvalue false))

(fn ConstructionScript)

(fn Toggle
  (Variables|Default|SetisWidgetInViewport (not (Variables|Default|GetisWidgetInViewport))))