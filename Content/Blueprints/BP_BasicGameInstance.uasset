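; Game instance that handles the transition from main menu to gameplay and provides inventory icon lookup.
; GameBeginning removes the main menu, hides the cursor, runs the WB_Lore intro widget and binds an event to its end.
; StartPlay blends the view to the player character and switches to game-only input.
; GetAssociatedImage maps an actor class through InventoryNameMap to its texture in the DTInventory data table.
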(fn GetAssociatedImage
  (params (ActorClass :type Actor%20Class%20Reference))
  (bind _inventorynamemap (Variables|Default|GetInventoryNameMap))
  (bind (_value _returnvalue) (Utilities|Map|Find _inventorynamemap ActorClass))
  (if _returnvalue
    (bind _texturereference (CallFunction|GetItemTexture (Variables|Default|GetDT_Inventory) _value))
    (return _texturereference)))

(fn GameBeginning
  ;[0.15 0.15 0.15 0.5] Remove menu
  (bind _foundwidgets (Widget|GetAllWidgetsOfClass "/Game/Widgets/MainMenu/WB_MainMenu.WB_MainMenu_C" true))
  (Widget|RemovefromParent (Utilities|Array|Get(acopy) _foundwidgets))
  ;[0.15 0.15 0.15 0.5] Lore
  (Variables|/Script/Engine.PlayerController|SetbShowMouseCursor (Game|GetPlayerController 0) false)
  (bind _returnvalue (UserInterface|CreateWidget "/Game/Widgets/LoreUI/WB_Lore.WB_Lore_C"))
  (UserInterface|Viewport|AddtoViewport _returnvalue 0)
  (Default|BeginLore _returnvalue)
  (EventDispatchers|BindEventtoOnEndIntro _returnvalue (EventDispatchers|CreateEvent :!event StartPlay)))

(fn StartPlay
  (Game|Player|SetViewTargetwithBlend (Game|GetPlayerController 0) (Game|GetPlayerCharacter 0) 1.0 "VTBlend_EaseInOut" 2.0 false)
  (Input|SetInputModeGameOnly (Game|GetPlayerController 0) false))